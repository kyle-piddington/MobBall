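; A clickable 3D menu button actor that opens the level named in its LevelLoad variable.
; The construction script writes ButtonText into its text render component.
; Cursor over and end-over events toggle a hover flag, and Tick smoothly interpolates the root's world scale between its original size and a slightly enlarged one.
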(event EventBeginPlay
  (Input|EnableInput (Game|GetPlayerController 0))
  (bind _output_get (Variables|Default|SetOrigSize (Transformation|GetActorScale3D)))
  (Variables|Default|SetBigSize (* _output_get 1.25)))

(event EventTick
  (params (DeltaSeconds :type Float%20%28single-precision%29))
  (bind _defaultsceneroot (Variables|Default|GetDefaultSceneRoot))
  (if (Variables|Default|GetMouseOver)
    (Variables|Default|SetTargSize (Variables|Default|GetBigSize))
    (else
      (bind _output_get (Variables|Default|SetTargSize (Variables|Default|GetOrigSize)))))
  (Transformation|SetWorldScale3D _defaultsceneroot (Math|Interpolation|VInterpTo (Transformation|GetWorldScale _defaultsceneroot) _output_get DeltaSeconds 3.0)))

(event MouseInput|EventActorBeginCursorOver
  (Variables|Default|SetMouseOver true))

(event MouseInput|EventActorOnClicked
  (params (ButtonPressed :type Key%20Structure :default "AnyKey"))
  (Game|OpenLevel(byName) (Variables|Default|GetLevelLoad)))

(event MouseInput|EventActorEndCursorOver
  (Variables|Default|SetMouseOver false))

(fn ConstructionScript
  (Rendering|Components|TextRender|SetText (Variables|Default|GetTextRender) (Variables|Default|GetButtonText)))